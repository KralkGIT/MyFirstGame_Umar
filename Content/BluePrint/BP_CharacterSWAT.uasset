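; BP_CharacterSWAT is a player character Blueprint that handles basic movement, looking and sprinting through Enhanced Input.
; BeginPlay casts the controller to BP_ThirdPersonController, adds the IMP_Char mapping context and sets walking speed.
; Movement follows control rotation, with pitch zeroed for forward input, while look input drives controller yaw and pitch.
; Sprint switches MaxWalkSpeed between sprint and walking speeds; crouch and jump events are empty stubs.
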(event `self.ReceiveBeginPlay`
  ; Movement
  (bind _asbp_third_person_controller (cast `/Game/BluePrint/BP_ThirdPersonController` (`self.GetController`)))
  (`EnhancedInputSubsystemInterface.AddMappingContext` (pcsubsystem `EnhancedInputLocalPlayerSubsystem` _asbp_third_person_controller) "/Game/Character/Basic_Shooter_Pack/Input/IMP_Char.IMP_Char" 0 (struct))
  (set `CharacterMovementComponent.MaxWalkSpeed` (`self.WalkingSpeed`) (`self.CharacterMovement`)))

(event `EnhancedInput|/Game/Character/Basic_Shooter_Pack/Input/IA_Movement`
  (params (ActionValue :type "Vector2D Structure") (ElapsedSeconds :type "Float (double-precision)") (TriggeredSeconds :type "Float (double-precision)") (InputAction :type "InputAction Object Reference" :default "/Game/Character/Basic_Shooter_Pack/Input/IA_Movement.IA_Movement"))
  (bind (_returnvalue_roll _returnvalue_pitch _returnvalue_yaw) (`KismetMathLibrary.BreakRotator` (`self.GetControlRotation`)))
  ; Movement
  (:`Triggered`
    (`self.AddMovementInput` (`KismetMathLibrary.GetRightVector` (`self.GetControlRotation`)) ActionValue_X)
    (`self.AddMovementInput` (`KismetMathLibrary.GetForwardVector` (`KismetMathLibrary.MakeRotator` _returnvalue_roll 0.0 _returnvalue_yaw)) ActionValue_Y)))

(event `EnhancedInput|/Game/Character/Basic_Shooter_Pack/Input/IA_Look`
  (params (ActionValue :type "Vector2D Structure") (ElapsedSeconds :type "Float (double-precision)") (TriggeredSeconds :type "Float (double-precision)") (InputAction :type "InputAction Object Reference" :default "/Game/Character/Basic_Shooter_Pack/Input/IA_Look.IA_Look"))
  ; Movement
  (:`Triggered`
    (`self.AddControllerYawInput` ActionValue_X)
    (`self.AddControllerPitchInput` ActionValue_Y)))

(event `EnhancedInput|/Game/Character/Basic_Shooter_Pack/Input/IA_Sprint`
  (params (ActionValue :type Boolean) (ElapsedSeconds :type "Float (double-precision)") (TriggeredSeconds :type "Float (double-precision)") (InputAction :type "InputAction Object Reference" :default "/Game/Character/Basic_Shooter_Pack/Input/IA_Sprint.IA_Sprint"))
  ; Movement
  (:`Started`
    (set `CharacterMovementComponent.MaxWalkSpeed` (`self.SprintSpeed`) (`self.CharacterMovement`)))
  (:`Completed`
    (set `CharacterMovementComponent.MaxWalkSpeed` (`self.WalkingSpeed`) (`self.CharacterMovement`))))

(event `EnhancedInput|/Game/Character/Basic_Shooter_Pack/Input/IA_Crouch`
  (params (ActionValue :type Boolean) (ElapsedSeconds :type "Float (double-precision)") (TriggeredSeconds :type "Float (double-precision)") (InputAction :type "InputAction Object Reference" :default "/Game/Character/Basic_Shooter_Pack/Input/IA_Crouch.IA_Crouch"))
  ; Movement
)

(event `EnhancedInput|/Game/Character/Basic_Shooter_Pack/Input/IA_Jump`
  (params (ActionValue :type "Vector2D Structure") (ElapsedSeconds :type "Float (double-precision)") (TriggeredSeconds :type "Float (double-precision)") (InputAction :type "InputAction Object Reference" :default "/Game/Character/Basic_Shooter_Pack/Input/IA_Jump.IA_Jump"))
  ; Movement
)

(fn `UserConstructionScript`)