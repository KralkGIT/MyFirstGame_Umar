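; BP_Score is a simple score counter Blueprint driven by a keyboard press.
; Pressing G while Score is below 100 raises it by a fixed step and prints an Indonesian confirmation message with the new value.
; Once the limit is reached, further presses only print that the score has been reached.
; BeginPlay and the construction script are empty.
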(event `Key|G`
  (params (Key :type "Key Structure"))
  (:`Pressed`
    (if (< (`self.Score`) 100)
      (`KismetSystemLibrary.PrintString` "Score DItambahkan")
      (set `self.Score` (+ (`self.Score`) 20))
      (`KismetSystemLibrary.PrintString` (`KismetStringLibrary.Conv_IntToString` (`self.Score`)))
      (else
        (`KismetSystemLibrary.PrintString` "Score Sudah Tercapai")))))

(fn `UserConstructionScript`)